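; BP_FakeKeyboardIncameraTracking is an actor that uses the keyboard to stand in for camera tracking in the IncameraStage project.
; It enables input from the first player controller on BeginPlay.
; While Enabled is set, the 1 and 2 keys nudge the referenced Camera1 actor backward or forward along world Y in fixed steps, one step per press.
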(event `self.ReceiveBeginPlay`
  (`self.EnableInput` (`GameplayStatics.GetPlayerController` 0)))

(event `self.ReceiveTick`
  (params (DeltaSeconds :type "Float (single-precision)")))

(event `Key|One`
  (params (Key :type "Key Structure"))
  (bind (_returnvalue_x _returnvalue_y _returnvalue_z) (`KismetMathLibrary.BreakVector` (`self.K2_GetActorLocation` (`self.Camera1`))))
  (:`Pressed`
    (if (`self.Enabled`)
      (`self.K2_SetActorLocation` (`self.Camera1`) (`KismetMathLibrary.MakeVector` _returnvalue_x (+ _returnvalue_y -5.0) _returnvalue_z) false false))))

(event `Key|Two`
  (params (Key :type "Key Structure"))
  (bind (_returnvalue_x _returnvalue_y _returnvalue_z) (`KismetMathLibrary.BreakVector` (`self.K2_GetActorLocation` (`self.Camera1`))))
  (:`Pressed`
    (if (`self.Enabled`)
      (`self.K2_SetActorLocation` (`self.Camera1`) (`KismetMathLibrary.MakeVector` _returnvalue_x (+ _returnvalue_y 5.0) _returnvalue_z) false false))))

(fn `UserConstructionScript`)
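; Debug-style Blueprint in IncameraStage that adjusts the render resolution of the nDisplay viewport "vp_1" at runtime.
; It enables input from the first player controller on BeginPlay.
; The 3 and 4 keys read the viewport's current buffer ratio through the display cluster API and step it down or up by a fixed amount, with no clamping in the graph.
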(event `self.ReceiveBeginPlay`
  (`self.EnableInput` (`GameplayStatics.GetPlayerController` 0)))

(event `Key|Three`
  (params (Key :type "Key Structure"))
  (bind _outapi (`DisplayClusterBlueprintLib.GetAPI`))
  (:`Pressed`
    (bind _outbufferratio (`DisplayClusterBlueprintAPI.GetBufferRatio` _outapi "vp_1"))
    (`DisplayClusterBlueprintAPI.SetBufferRatio` _outapi "vp_1" (- _outbufferratio 0.1))))

(event `Key|Four`
  (params (Key :type "Key Structure"))
  (bind _outapi (`DisplayClusterBlueprintLib.GetAPI`))
  (:`Pressed`
    (bind _outbufferratio (`DisplayClusterBlueprintAPI.GetBufferRatio` _outapi "vp_1"))
    (`DisplayClusterBlueprintAPI.SetBufferRatio` _outapi "vp_1" (+ _outbufferratio 0.1))))

(fn `UserConstructionScript`)
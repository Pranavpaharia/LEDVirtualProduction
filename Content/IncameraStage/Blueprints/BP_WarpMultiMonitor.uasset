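; BP_WarpMultiMonitor is an actor that sets up warp meshes for a three-screen multi-monitor display.
; On BeginPlay it assigns its left, center and right screen mesh components to viewports vp_1, vp_2 and vp_3 through an API call.
; All three assignments use the actor's root component as the origin.
; Tick, overlap and the construction script are empty.
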(event `self.ReceiveBeginPlay`
  ;[1 1 1] Setup warp
  (`PicpProjectionBlueprintAPI.AssignWarpMeshToViewport` (`PicpProjectionIBlueprintLib.GetAPI`) "vp_1" (`self.Screen_left`) (`self.root`))
  (`PicpProjectionBlueprintAPI.AssignWarpMeshToViewport` (`PicpProjectionIBlueprintLib.GetAPI`) "vp_2" (`self.Screen_center`) (`self.root`))
  (`PicpProjectionBlueprintAPI.AssignWarpMeshToViewport` (`PicpProjectionIBlueprintLib.GetAPI`) "vp_3" (`self.Screen_right`) (`self.root`)))

(fn `UserConstructionScript`)
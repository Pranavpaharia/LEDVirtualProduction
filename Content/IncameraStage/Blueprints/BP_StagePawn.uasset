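; Flyable pawn for an in-camera LED stage that moves the stage origin and drives the tracked cine camera.
; Input axes fly it along its camera's axes and turn the view.
; Each tick it copies its transform to the BP_LEDStageOriginView actor and applies Vive VRPN tracker pose to the CineCameraActor's relative transform.
; Pressing R stores the current tracker location as the calibration offset subtracted from camera position.
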(event `InputAxis|LookUpRate`
  (params (AxisValue :type "Float (single-precision)"))
  (`self.AddControllerPitchInput` AxisValue))

(event `InputAxis|TurnRate`
  (params (AxisValue :type "Float (single-precision)"))
  (`self.AddControllerYawInput` AxisValue))

(event `self.ReceiveBeginPlay`
  (bind _returnvalue (`GameplayStatics.GetActorOfClass` "/Script/CinematicCamera.CineCameraActor"))
  (set `self.CineCam` _returnvalue)
  (bind _returnvalue_2 (`GameplayStatics.GetActorOfClass` "/Game/IncameraStage/Blueprints/BP_LEDStageOriginView.BP_LEDStageOriginView_C"))
  (set `self.Origin LEDWall` _returnvalue_2)
  (bind _outactors (`GameplayStatics.GetAllActorsOfClass` "/Script/Engine.PlayerStart"))
  (set `self.SpotList` _outactors))

(event `InputAxis|MoveUp`
  (params (AxisValue :type "Float (single-precision)"))
  (`PawnMovementComponent.AddInputVector` (`self.FloatingPawnMovement`) (* (`SceneComponent.GetUpVector` (`self.Camera`)) (* AxisValue 100.0)) false))

(event `InputAxis|MoveRight`
  (params (AxisValue :type "Float (single-precision)"))
  (`PawnMovementComponent.AddInputVector` (`self.FloatingPawnMovement`) (* (`SceneComponent.GetRightVector` (`self.Camera`)) (* AxisValue 100.0)) false))

(event `self.ReceiveTick`
  (params (DeltaSeconds :type "Float (single-precision)"))
  (bind _outapi (`DisplayClusterBlueprintLib.GetAPI`))
  (bind _origin_ledwall (`self.Origin LEDWall`))
  (bind _rootcomponent (`Actor.RootComponent` (`self.CineCam`)))
  (bind _location (`DisplayClusterBlueprintAPI.GetTrackerLocation` _outapi "ViveVRPN" 0))
  (bind _rotation (`DisplayClusterBlueprintAPI.GetTrackerQuat` _outapi "ViveVRPN" 0))
  (`SceneComponent.K2_SetRelativeLocation` _rootcomponent (- _location (`self.TrackerOffsetCalibration`)) false false)
  (`SceneComponent.K2_SetRelativeRotation` _rootcomponent (`KismetMathLibrary.Quat_Rotator` _rotation) false false)
  (`/Engine/EditorBlueprintResources/StandardMacros.IsValid` _origin_ledwall
    (:`Is Valid`
      (`self.K2_SetActorTransform` _origin_ledwall (`self.GetTransform`) false false))))

(event `Key|R`
  (params (Key :type "Key Structure"))
  (:`Pressed`
    (set `self.TrackerOffsetCalibration` (stale `self.ReceiveTick` _location))))

(event `Key|E`
  (params (Key :type "Key Structure")))

(event `InputAxis|MoveForward`
  (params (AxisValue :type "Float (single-precision)"))
  (`PawnMovementComponent.AddInputVector` (`self.FloatingPawnMovement`) (* (`SceneComponent.GetForwardVector` (`self.Camera`)) (* AxisValue 100.0)) false))

(event `Key|W`
  (params (Key :type "Key Structure")))

(fn `UserConstructionScript`)